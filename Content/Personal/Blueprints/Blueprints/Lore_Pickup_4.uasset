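; Lore pickup actor, the fourth entry, that loops a spin-and-bob sequence from BeginPlay until something overlaps it.
; The first overlap by any actor destroys the pickup and plays a UI hover sound at world origin.
; If that actor is an AGM_Character, it then shows LoreEntry_4_Widget, with a timed removal scheduled on the already destroyed actor.
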(event `self.ReceiveBeginPlay`
  (`MovieSceneSequencePlayer.PlayLooping` (`ActorSequenceComponent.SequencePlayer` (`self.SpinBob`)) -1))

(event `self.ReceiveActorBeginOverlap`
  (params (OtherActor :type "Actor Object Reference"))
  (`/Engine/EditorBlueprintResources/StandardMacros.DoOnce` false
    (:`Completed`
      (`|ExecutionSequence`
        (:`then_0`
          (`self.K2_DestroyActor`)
          (`GameplayStatics.PlaySoundAtLocation` "/Game/Personal/Audio/UI/UI_Hover_Cue.UI_Hover_Cue" (0.0 0.0 0.0) (struct) 1.0 1.0 0.0 null null null))
        (:`then_1`
          (cast `/Game/Personal/Blueprints/Blueprints/AGM_Character` OtherActor)
          (bind _returnvalue (`|CreateWidget` "/Game/Personal/Art/UI/Lore/LoreEntry_4_Widget.LoreEntry_4_Widget_C"))
          (`UserWidget.AddToViewport` _returnvalue 0)
          (`KismetSystemLibrary.Delay` 10.5)
          (`Widget.RemoveFromParent` _returnvalue))))))

(fn `UserConstructionScript`)