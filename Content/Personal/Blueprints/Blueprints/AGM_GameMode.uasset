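; AGM_GameMode is a game mode Blueprint that holds back player input at the start and runs the gameplay timer.
; BeginPlay disables character input, waits through a fixed delay, then restores input, shows the AGM_HUD widget and sets StartPlay.
; Tick then advances minute, second and sub-second counters through a short Delay, so timing depends on frame rate.
; Two countdown sequences, one widget-based and one looping, are left unconnected.
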(event `self.ReceiveBeginPlay`
  (bind _returnvalue (`GameplayStatics.GetPlayerCharacter` 0))
  ;[1 1 1] Play Delay
  (bind _asagm_character (cast `/Game/Personal/Blueprints/Blueprints/AGM_Character` _returnvalue))
  (`self.DisableInput` _asagm_character null)
  (`KismetSystemLibrary.Delay` 8.3)
  (`self.EnableInput` _returnvalue null)
  ;[1 1 1] Show HUD
  (bind _returnvalue_2 (`|CreateWidget` "/Game/Personal/Art/UI/AGM_HUD.AGM_HUD_C"))
  (`UserWidget.AddToViewport` _returnvalue_2 0)
  (set `self.Start Play` true))

(event `self.ReceiveTick`
  (params (DeltaSeconds :type "Float (single-precision)"))
  ;[1 1 1] Gameplay Timer
  (if (`self.Start Play`)
    (`KismetSystemLibrary.Delay` 0.01)
    (set `self.Time MSec` (+ (`self.Time MSec`) 1))
    (if (> (`self.Time MSec`) 59)
      (set `self.Time Sec` (+ (`self.Time Sec`) 1))
      (set `self.Time MSec` 0)
      (if (> (`self.Time Sec`) 59)
        (set `self.Time Min` (+ (`self.Time Min`) 1))
        (set `self.Time Sec` 0)))))

(fn `UserConstructionScript`)