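; Lore pickup actor for the second lore entry, animated by a looping SpinBob sequence from BeginPlay.
; The first overlap by any actor destroys the pickup, plays a fade sound at world origin and sets Lore2IsCollected.
; Only afterwards does it cast to AGM_Character to show the LoreEntry_2_Widget.
; The widget's timed removal sits behind a Delay on the already destroyed actor.
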(event `self.ReceiveBeginPlay`
  (set `self.Lore2_IsCollected?` false)
  (`MovieSceneSequencePlayer.PlayLooping` (`ActorSequenceComponent.SequencePlayer` (`self.SpinBob`)) -1))

(event `self.ReceiveActorBeginOverlap`
  (params (OtherActor :type "Actor Object Reference"))
  (`/Engine/EditorBlueprintResources/StandardMacros.DoOnce` false
    (:`Completed`
      (`|ExecutionSequence`
        (:`then_0`
          (`self.K2_DestroyActor`)
          (`GameplayStatics.PlaySoundAtLocation` "/Game/Personal/Audio/UI/AGM_FadeSound_Cue.AGM_FadeSound_Cue" (0.0 0.0 0.0) (struct) 1.0 1.0 0.0 null null null)
          (set `self.Lore2_IsCollected?` true))
        (:`then_1`
          (cast `/Game/Personal/Blueprints/Blueprints/AGM_Character` OtherActor)
          (bind _returnvalue (`|CreateWidget` "/Game/Personal/Art/UI/Lore/LoreEntry_2_Widget.LoreEntry_2_Widget_C"))
          (`UserWidget.AddToViewport` _returnvalue 0)
          (`KismetSystemLibrary.Delay` 10.5)
          (`Widget.RemoveFromParent` _returnvalue))))))

(fn `UserConstructionScript`)