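; Level-end trigger that, when the player character overlaps it, stops play and shows the leaderboard end-game screen.
; It flags the game as ended, captures the game mode's timer, plays a brief fade widget, then pauses with UI-only input.
; Collected lore and ammo pickups from the pickup manager light up pips on the screen.
; The time and both collection arrays are inserted as a score into a loaded or newly created save game.
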(event `self.ReceiveActorBeginOverlap`
  (params (OtherActor :type "Actor Object Reference"))
  (bind _returnvalue (`GameplayStatics.GetPlayerController` 0))
  (bind _currentsavegame (`self.CurrentSaveGame`))
  (bind _as_agm_game_mode (`self.As AGM Game Mode`))
  (bind _asagm_character (cast `/Game/Personal/Blueprints/Blueprints/AGM_Character` OtherActor))
  (set `self.As AGM Character` _asagm_character)
  (bind _asagm_game_mode (cast `/Game/Personal/Blueprints/Blueprints/AGM_GameMode` (`GameplayStatics.GetGameMode`)))
  (set `self.As AGM Game Mode` _asagm_game_mode)
  (set `self.GameHasEnded` true)
  (set `self.Time Min` (`/Game/Personal/Blueprints/Blueprints/AGM_GameMode.Time Min` _as_agm_game_mode))
  (set `self.Time Sec` (`/Game/Personal/Blueprints/Blueprints/AGM_GameMode.Time Sec` _as_agm_game_mode))
  (set `self.Time MSec` (`/Game/Personal/Blueprints/Blueprints/AGM_GameMode.Time MSec` _as_agm_game_mode))
  (bind _returnvalue_2 (`|CreateWidget` "/Game/Personal/UI/Other/OffWhiteFadeWidget.OffWhiteFadeWidget_C"))
  (`UserWidget.AddToViewport` _returnvalue_2 0)
  (`KismetSystemLibrary.Delay` 1.0)
  (`|ExecutionSequence`
    (:`then_0`
      (`Widget.RemoveFromParent` _returnvalue_2))
    (:`then_1`
      (`GameplayStatics.SetGamePaused` true)
      (bind _returnvalue_3 (`|CreateWidget` "/Game/Personal/UI/Menus/Lboard_EndGame_Widget.Lboard_EndGame_Widget_C" _returnvalue))
      (bind _output_get (set `self.EndGameUIRef` _returnvalue_3))
      (`UserWidget.AddToViewport` _output_get 0)
      (`WidgetBlueprintLibrary.SetInputMode_UIOnlyEx` _returnvalue null)
      (set `PlayerController.bShowMouseCursor` true _returnvalue)
      (`TextBlock.SetText` (`/Game/Personal/UI/Menus/Lboard_EndGame_Widget.TimeBindText` (`self.EndGameUIRef`)) (`|FormatText` "{Min} : {Sec} : {MSec}" (`KismetTextLibrary.Conv_IntToText` (`self.Time Min`) false true 2 2) (`KismetTextLibrary.Conv_IntToText` (`self.Time Sec`) false true 2 2) (`KismetTextLibrary.Conv_IntToText` (`self.Time MSec`) false true 2 2)))
      (`self.LorePipCheck`)
      (`self.AmmoPipCheck`)
      (bind _returnvalue_4 (`GameplayStatics.DoesSaveGameExist` "Slot"))
      (if _returnvalue_4
        (bind _returnvalue_5 (`GameplayStatics.LoadGameFromSlot` "Slot"))
        (bind _aslb_save_game (cast `/Game/Personal/Leaderboard/LB_SaveGame` _returnvalue_5)
          (:`then`
            (set `self.CurrentSaveGame` _aslb_save_game))
          (:`CastFailed`
            (bind _returnvalue_6 (`GameplayStatics.CreateSaveGameObject` "/Game/Personal/Leaderboard/LB_SaveGame.LB_SaveGame_C" :!label _label))
            (set `self.CurrentSaveGame` _returnvalue_6)))
        (else
          (goto _label)))
      (`/Game/Personal/Leaderboard/LB_SaveGame.Insert` _currentsavegame (make `/Game/Personal/Leaderboard/ST_Score` (`self.Time Min`) (`self.Time Sec`) (`self.Time MSec`) (`self.AmmoBools`) (`self.LoreBools`)))
      (bind _returnvalue_7 (`GameplayStatics.SaveGameToSlot` _currentsavegame "Slot"))
      (`KismetSystemLibrary.PrintString` (`KismetStringLibrary.Concat_StrStr` "Has Saved? " (`KismetStringLibrary.Conv_BoolToString` _returnvalue_7))))))

(event `AmmoPipCheck`
  ;[1 1 1] Ammo/Lore Pips
  (for (_array_element _array_index) (`/Game/Personal/Blueprints/Blueprints/PickUps/PickUpManager.AmmoCollection` (`/Game/Personal/Blueprints/Blueprints/AGM_GameMode.PickUpManagerRef` (`self.As AGM Game Mode`)))
    (if (`/Game/Personal/Blueprints/Blueprints/PickUps/Ammo_Pickup.HasBeenPickedUp?` _array_element)
      (`KismetArrayLibrary.Array_Set` (`self.AmmoBools`) _array_index true)
      (bind _output (`|GetArrayItem` (`/Game/Personal/UI/Menus/Lboard_EndGame_Widget.AmmoPips` (`self.EndGameUIRef`)) _array_index))
      (if (not (`KismetSystemLibrary.IsValid` _output))
        (`/Game/Personal/UI/Menus/Lboard_EndGame_Widget.CreatePipArrays` (`self.EndGameUIRef`)))
      (`Image.SetColorAndOpacity` _output (struct :`R` 0.999643 :`G` 1.0 :`B` 0.916018 :`A` 1.0)))))

(event `LorePipCheck`
  (bind _lorebools (`self.LoreBools`))
  ;[1 1 1] Ammo/Lore Pips
  (for (_array_element _array_index) (`/Game/Personal/Blueprints/Blueprints/PickUps/PickUpManager.LoreCollection` (`/Game/Personal/Blueprints/Blueprints/AGM_GameMode.PickUpManagerRef` (`self.As AGM Game Mode`)))
    (if (`/Game/Personal/Blueprints/Blueprints/PickUps/Lore_Pickup_1.HasBeenIsCollected?` _array_element)
      (`KismetArrayLibrary.Array_Set` _lorebools _array_index true)
      (`KismetSystemLibrary.PrintString` (`KismetStringLibrary.Concat_StrStr` (`KismetStringLibrary.Conv_IntToString` _array_index) " = " (`KismetStringLibrary.Conv_BoolToString` (`|GetArrayItem` _lorebools _array_index))))
      (bind _output (`|GetArrayItem` (`/Game/Personal/UI/Menus/Lboard_EndGame_Widget.LorePips` (`self.EndGameUIRef`)) _array_index))
      (if (not (`KismetSystemLibrary.IsValid` _output))
        (`/Game/Personal/UI/Menus/Lboard_EndGame_Widget.CreatePipArrays` (`self.EndGameUIRef`)))
      (`Image.SetColorAndOpacity` _output (struct :`R` 0.999643 :`G` 1.0 :`B` 0.916018 :`A` 1.0)))))

(fn `UserConstructionScript`)