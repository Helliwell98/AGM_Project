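; Lore pickup actor that shows a piece of lore text on screen when the AGM character touches it.
; A looping sequence player, SpinBob, animates it from BeginPlay.
; A DoOnce-gated overlap plays sound and particles, disables and hides the pickup, and shows a LoreEntry widget filled with LoreToGive, removed after a delay.
; Reset restores visibility, collision and the gate so it can be collected again.
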(event `self.ReceiveBeginPlay`
  (set `self.HasBeenIsCollected?` false)
  (`MovieSceneSequencePlayer.PlayLooping` (`ActorSequenceComponent.SequencePlayer` (`self.SpinBob`)) -1))

(event `self.coll.OnComponentBeginOverlap`
  (params (OverlappedComponent :type "PrimitiveComponent Object Reference") (OtherActor :type "Actor Object Reference") (OtherComp :type "PrimitiveComponent Object Reference") (OtherBodyIndex :type Integer) (bFromSweep :type Boolean) (SweepResult :type "HitResult Structure (by ref)"))
  (bind _asagm_character (cast `/Game/Personal/Blueprints/Blueprints/AGM_Character` OtherActor))
  (set `self.As AGM Character` _asagm_character)
  (`/Engine/EditorBlueprintResources/StandardMacros.DoOnce` false :!label _label
    (:`Completed`
      (`|ExecutionSequence`
        (:`then_0`
          (`GameplayStatics.PlaySound2D` "/Game/Personal/Audio/UI/AGM_FadeSound_Cue.AGM_FadeSound_Cue" 1.0 1.0 0.0 null null)
          (`GameplayStatics.SpawnEmitterAtLocation` null (`SceneComponent.K2_GetComponentLocation` (`self.Sphere`)))
          (set `self.HasBeenIsCollected?` true)
          (`PrimitiveComponent.SetCollisionEnabled` (`self.coll`) "NoCollision")
          (`self.SetActorHiddenInGame` true))
        (:`then_1`
          (bind _returnvalue (`|CreateWidget` "/Game/Personal/UI/Lore/LoreEntry_1_Widget.LoreEntry_1_Widget_C"))
          (`TextBlock.SetText` (`/Game/Personal/UI/Lore/LoreEntry_1_Widget.LOREWIDGET` _returnvalue) (`self.LoreToGive`))
          (`UserWidget.AddToViewport` _returnvalue 0)
          (`KismetSystemLibrary.Delay` 10.5)
          (`Widget.RemoveFromParent` _returnvalue))))))

(event `Reset`
  (`KismetSystemLibrary.PrintString` "RESET")
  (set `self.HasBeenIsCollected?` false)
  (`PrimitiveComponent.SetCollisionEnabled` (`self.coll`) "QueryAndPhysics")
  (`self.SetActorHiddenInGame` false)
  (goto _label :!via `Reset`))

(fn `UserConstructionScript`)