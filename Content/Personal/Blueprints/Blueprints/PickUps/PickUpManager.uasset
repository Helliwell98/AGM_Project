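; PickUpManager is a manager actor that resets the level's lore and ammo pickups on request.
; On BeginPlay it registers itself as the PickUpManagerRef on the AGM_GameMode, giving other systems access to it.
; Its ResetPickUps event loops over the LoreCollection and AmmoCollection arrays and calls Reset on each element.
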(event `self.ReceiveBeginPlay`
  (bind _asagm_game_mode (cast `/Game/Personal/Blueprints/Blueprints/AGM_GameMode` (`GameplayStatics.GetGameMode`)))
  (set `/Game/Personal/Blueprints/Blueprints/AGM_GameMode.PickUpManagerRef` self _asagm_game_mode))

(event `ResetPickUps`
  (for _array_element (`self.LoreCollection`)
    (`/Game/Personal/Blueprints/Blueprints/PickUps/Lore_Pickup_1.Reset` _array_element))
  (for _array_element_2 (`self.AmmoCollection`)
    (`/Game/Personal/Blueprints/Blueprints/PickUps/Ammo_Pickup.Reset` _array_element_2)))

(fn `UserConstructionScript`)