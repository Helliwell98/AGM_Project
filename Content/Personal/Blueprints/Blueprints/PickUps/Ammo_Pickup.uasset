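; Ammo pickup actor that permanently raises the player's ammo capacity and refills their ammo.
; It loops a SpinBob sequence from BeginPlay.
; When an AGM_Character overlaps the collision, it increments MaxAmmo, fills CurrentAmmo, plays a reload sound and spawns an emitter.
; It then hides and disables collision instead of being destroyed, so a Reset event can restore it.
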(event `self.ReceiveBeginPlay`
  (`MovieSceneSequencePlayer.PlayLooping` (`ActorSequenceComponent.SequencePlayer` (`self.SpinBob`)) -1))

(event `self.coll.OnComponentBeginOverlap`
  (params (OverlappedComponent :type "PrimitiveComponent Object Reference") (OtherActor :type "Actor Object Reference") (OtherComp :type "PrimitiveComponent Object Reference") (OtherBodyIndex :type Integer) (bFromSweep :type Boolean) (SweepResult :type "HitResult Structure (by ref)"))
  (bind _asagm_character (cast `/Game/Personal/Blueprints/Blueprints/AGM_Character` OtherActor))
  (bind _output_get (set `/Game/Personal/Blueprints/Blueprints/AGM_Character.Max Ammo` (+ (stale _output_get) 1) _asagm_character))
  (set `/Game/Personal/Blueprints/Blueprints/AGM_Character.Current Ammo` _output_get _asagm_character)
  (`GameplayStatics.PlaySound2D` "/Game/Personal/Audio/Gun/Relaod_Cue.Relaod_Cue" 1.1 1.0 0.0 null null)
  (`GameplayStatics.SpawnEmitterAtLocation` null (`SceneComponent.K2_GetComponentLocation` (`self.Sphere`)))
  (set `self.HasBeenPickedUp?` true)
  (`PrimitiveComponent.SetCollisionEnabled` (`self.coll`) "NoCollision")
  (`self.SetActorHiddenInGame` true))

(event `Reset`
  (set `self.HasBeenPickedUp?` false)
  (`PrimitiveComponent.SetCollisionEnabled` (`self.coll`) "QueryAndPhysics")
  (`self.SetActorHiddenInGame` false))

(fn `UserConstructionScript`)